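; RespawnBP is a checkpoint actor that sets where the Ybot character respawns.
; On BeginPlay it stores the level's Ybot transform as SpawnLocation in OldWorld_GameMode, giving an initial spawn point.
; When a Ybot overlaps its Box, it overwrites SpawnLocation with that character's current transform and makes its Fire and PointLight visible to mark activation.
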(event OnComponentBeginOverlap(Box)
  (params (OverlappedComponent :type Primitive%20Component%20Object%20Reference) (OtherActor :type Actor%20Object%20Reference) (OtherComp :type Primitive%20Component%20Object%20Reference) (OtherBodyIndex :type Integer) (bFromSweep :type Boolean) (SweepResult :type Hit%20Result%20Structure%20%28by%20ref%29))
  (bind _asybot (Utilities|Casting|CastToybot OtherActor))
  (bind _asold_world_game_mode (Utilities|Casting|CastToOldWorld_GameMode (Game|GetGameMode)))
  (Variables|/Game/Blueprints/OldWorld_GameMode.OldWorld_GameMode_C|SetSpawnLocation _asold_world_game_mode (Transformation|GetActorTransform _asybot))
  (Rendering|SetVisibility (Variables|Default|GetFire) true false))

(event EventBeginPlay
  (bind _returnvalue (Actor|GetActorOfClass "/Game/Blueprints/ybot.ybot_C"))
  (bind _output_get (Variables|Default|SetYbot _returnvalue))
  (bind _asold_world_game_mode (Utilities|Casting|CastToOldWorld_GameMode (Game|GetGameMode)))
  (Variables|/Game/Blueprints/OldWorld_GameMode.OldWorld_GameMode_C|SetSpawnLocation _asold_world_game_mode (Transformation|GetActorTransform _output_get)))

(fn ConstructionScript)