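; Level transition trigger that sends the player back to the previous numbered level.
; When a ybot overlaps its Box, it checks the current level name and does nothing further on L1.
; Otherwise it fades the camera, waits briefly, then opens the previous level, whose name it derives by parsing the number after the "L" prefix and subtracting one.
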(event OnComponentBeginOverlap(Box)
  (params (OverlappedComponent :type Primitive%20Component%20Object%20Reference) (OtherActor :type Actor%20Object%20Reference) (OtherComp :type Primitive%20Component%20Object%20Reference) (OtherBodyIndex :type Integer) (bFromSweep :type Boolean) (SweepResult :type Hit%20Result%20Structure%20%28by%20ref%29))
  (Utilities|Casting|CastToybot OtherActor)
  (bind _returnvalue (Game|GetCurrentLevelName true))
  (if (not (Utilities|Enum|Equal(Enum) _returnvalue "L1"))
    (CameraFades|StartCameraFade :self (Game|GetPlayerCameraManager 0) :FromAlpha 0.0 :ToAlpha 2.0 :Duration 1.0)
    (Utilities|FlowControl|Delay 0.9)
    (Game|OpenLevel(byName) (Utilities|String|StringToName (Utilities|String|Append "L" (Utilities|String|ToString(Integer) (- (Math|Conversions|ToInteger(Byte) (Utilities|String|GetSubstring _returnvalue 1 (Utilities|String|Len _returnvalue))) 1)))))))

(fn ConstructionScript)