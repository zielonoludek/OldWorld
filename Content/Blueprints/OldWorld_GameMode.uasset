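; OldWorld_GameMode is a game mode Blueprint that respawns the player's Ybot character whenever it is destroyed.
; On BeginPlay it casts player 0's character to Ybot and binds to its OnDestroyed event.
; When that fires, a zero-length Delay precedes spawning a new Ybot at the SpawnLocation transform and having player controller 0 possess it.
; The Respawn event then rebinds to the new character, so the cycle repeats.
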(event Custom|OnDestroyed_
  (params (DestroyedActor :type Actor%20Object%20Reference))
  (Utilities|FlowControl|Delay 0.0)
  (bind _returnvalue (Game|SpawnActorfromClass "/Game/Blueprints/ybot.ybot_C" (Variables|Default|GetSpawnLocation) "Undefined" 0 0))
  (Pawn|Possess (Game|GetPlayerController 0) _returnvalue)
  (CallFunction|Respawn))

(event Custom|Respawn
  (bind _asybot (Utilities|Casting|CastToybot (Game|GetPlayerCharacter 0)))
  (Game|BindEventtoOnDestroyed _asybot (delegate Custom|OnDestroyed_)))

(event EventBeginPlay
  (bind _asybot (Utilities|Casting|CastToybot (Game|GetPlayerCharacter 0)))
  (Game|BindEventtoOnDestroyed _asybot (delegate Custom|OnDestroyed_)))

(fn ConstructionScript)